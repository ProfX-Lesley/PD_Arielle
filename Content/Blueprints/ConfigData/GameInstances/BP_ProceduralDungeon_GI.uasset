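; Game Instance that builds a procedural dungeon from a seeded random stream, randomizing the seed when it is zero.
; It spawns a starter room, then attaches extension rooms at random endpoints on a timer, retrying when collision boxes overlap.
; Overlapping check boxes identify connected endpoints; the rest get caps, then an exit spawns and the NavMesh bounds are fitted and rebuilt.
; Main menu mode instead clears and regenerates the dungeon in a slower loop.
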(event Custom|NavMeshSetup
  (bind _returnvalue (Actor|GetActorOfClass "/Script/NavigationSystem.NavMeshBoundsVolume"))
  (Variables|Default|SetNavMeshRef _returnvalue)
  (bind _outactors (Actor|GetAllActorsOfClasswithTag "/Game/Blueprints/Actors/DungeonRooms/BP_Room_Master.BP_Room_Master_C" "DungeonRoom"))
  (bind _output_get (Variables|Default|SetAllRooms _outactors))
  (for _array_element _output_get
    (|CalculateTempNavMeshExtents _array_element)
    (|CalculateFinalDungeonExtents))
  (|CalculateNavMeshCenter&Scale)
  (|ApplyNavMeshCenter&Scale)
  (|RebuildNavMesh)
  (CallFunction|RoomRoulette))

(event Custom|RoomRoulette)

(event EventInitializeDungeonIF
  (CallFunction|VariablesReset)
  (CallFunction|ProcessSeedInput)
  (Utilities|PrintExtentions)
  (if (Variables|Default|GetIsMainMenu?_GI)
    (bind _output_get (Variables|Default|SetBuildDelay 1.0))
    (CallFunction|GenerateStarterRoom)
    (Utilities|FlowControl|Delay _output_get)
    (CallFunction|GenerateExtentionRoom)
    (else
      (Variables|Default|SetBuildDelay 0.01)
      (CallFunction|GenerateStarterRoom)
      (CallFunction|GenerateExtentionRoom))))

(fn ProcessSeedInput
  (bind _seedstream (Variables|Default|GetSeedStream))
  (if (== (Variables|Default|GetLoadingSeed) 0) ; If the user inputted 0 as their\ndesired seed, then it will ignore\nthe input, and the seed will be\nrandomized.\n\nIf the user did not input 0,\nthen the inputted number will be\nset as the seed number moving forward.
    (Class|KismetMathLibrary|SeedRandomStream _seedstream) ; Similar to a variable Setter, but with\nmore functionality.\nThis sets the random seed to be a\nrandom value.
    (Variables|Default|SetLoadingSeed (.initialseed (Variables|Default|GetSeedStream))) ; Used as a reference of the seed...
    (else
      (Math|Random|SetRandomStreamSeed _seedstream (Variables|Default|GetLoadingSeed)) ; Also similar to a variable setter\nwith more functionality.\nLooks at the User's inputted number,\nthen sets it as the random seed.
    )))

(fn GenerateStarterRoom
  (bind _returnvalue (Game|SpawnActorfromClass (CallFunction|RandomizeStartRoom) (Variables|Default|GetStartRoomSpawnPoint) "Undefined" "MultiplyWithRoot" 0 0)) ; Spawns in the Starting Room
  (Variables|Default|SetAllEndPoints (Variables|Default|GetAllEndPoints))
  (Utilities|Array|AppendArray (Variables|Default|GetAllEndPoints) (Components|GetChildrenComponents (Variables|/Game/Blueprints/Actors/DungeonRooms/BP_Room_Master.BP_Room_Master_C|GetEndPoints_Grp _returnvalue) false))
  (return))

(fn RandomizeStartRoom
  (bind _startroomclasses (Variables|Default|GetStartRoomClasses))
  (return (Utilities|Array|Get(acopy) _startroomclasses (Math|Random|RandomIntegerinRangefromStream (Variables|Default|GetSeedStream) 0 (- (Utilities|Array|Length _startroomclasses) 1)))))

(fn VariablesReset
  (Utilities|Array|Clear (Variables|Default|GetAllEndPoints))
  (Variables|Default|SetExtensions (- (Variables|Default|GetTotalRooms) 1))
  (Variables|Default|SetCurrentRoom 0)
  (Variables|Default|SetStartRoomSpawnPoint ""))

(fn GenerateExtentionRoom
  (if (> (Variables|Default|GetExtensions) 0) :!label _label
    (|GenerateRoom
      (:Success
        (Utilities|Time|SetTimerbyFunctionName 0 "Generate Extention Room" (Variables|Default|GetBuildDelay))
        (Development|PrintString (Utilities|String|ToString(Integer) (Variables|Default|GetExtensions))))
      (:Fail
        (goto _label)))
    (elif (Variables|Default|GetIsMainMenu?_GI) ; Is this the Main Menu?
      (CallFunction|ClearCurrentDungeon)
      (CallFunction|InitializeDungeonIF)
      (else
        (Development|PrintString "Extensions Complete!")
        (Utilities|GenerateEndCheckBoxes)
        (Utilities|ProcessValidEndPoints)
        (Utilities|GenerateRoomCaps)
        (Utilities|CleanUpEndCheckBoxes)
        (Utilities|GenerateExit)
        (CallFunction|NavMeshSetup)))))

(fn ClearCurrentDungeon
  (Variables|Default|SetLoadingSeed 0)
  (Utilities|Array|Clear (Variables|Default|GetCurrentOverlappedComponents))
  (CallFunction|VariablesReset)
  (bind _outactors (Actor|GetAllActorsOfClass "/Game/Blueprints/Actors/DungeonRooms/BP_Room_Master.BP_Room_Master_C"))
  (for _array_element _outactors
    (Actor|DestroyActor _array_element))
  (bind _outactors_2 (Actor|GetAllActorsOfClass "/Game/Blueprints/Actors/DungeonRooms/BP_RoomCap.BP_RoomCap_C"))
  (for _array_element_2 _outactors_2
    (Actor|DestroyActor _array_element_2))
  (Utilities|Platform|CollectGarbage))